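; Gameplay ability that triggers Berserk on its owning avatar.
; On activation it commits, plays the Berserk montage and waits for the Ability.Berserk gameplay event.
; When the event arrives, it applies the associated gameplay effect to the owner, executes the Berserk gameplay cue attached to the avatar's root component, and ends.
; Montage completion and interruption are not handled, so the ability ends only through that event path.
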(event Ability|EventActivateAbility
  (bind _returnvalue (Ability|GetAvatarActorfromActorInfo))
  (bind _returnvalue_2 (Ability|GetAvatarActorfromActorInfo))
  (bind _returnvalue_3 (Ability|GetAbilitySystemComponent _returnvalue_2))
  (Ability|CommitAbility)
  (|PlayMontageandWaitProxy "None" "/Game/Assets/Alien/Animations/AnimationMontages/AM_Berserk.AM_Berserk" 1.0 "None" true 1.0 0.0 false
    (:then
      (Ability|Tasks|WaitGameplayEvent "(TagName=\"Ability.Berserk\")" 0
        (:EventReceived
          (Ability|ApplyGameplayEffectSpecToOwner (GameplayEffects|MakeOutgoingSpec _returnvalue_3 (Variables|Default|GetAssociatedGameplayEffect) 1.0 (GameplayEffects|MakeEffectContext _returnvalue_3)))
          (Class|GameplayAbility|ExecuteGameplayCuewithParams "(TagName=\"GameplayCue.Berserk\")" (Ability|GameplayCue|MakeGameplayCueParameters :Instigator _returnvalue :TargetAttachComponent (Variables|/Script/Engine.Actor|GetRootComponent _returnvalue)))
          (Ability|EndAbility))))))